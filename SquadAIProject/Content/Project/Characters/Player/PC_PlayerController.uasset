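; Player controller for the player character that sets up Enhanced Input and the in-game HUD.
; On BeginPlay it adds the IMC_Player mapping context to the local player's Enhanced Input subsystem.
; It then casts the controlled pawn to BP_PlayerBase, caches it as ControlledPlayer, and calls InitUI to create and show the WB_InGameUI widget, which only happens if that cast succeeds.
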(event Custom|Init%20UI
  (bind _returnvalue (UserInterface|CreateWidget "/Game/Project/UserInterfacce/ScreenSpace/In_Game/WB_InGameUI.WB_InGameUI_C"))
  (bind _output_get (Variables|Default|SetIn%20Game%20UI _returnvalue))
  (UserInterface|Viewport|AddtoViewport _output_get 0))

(event EventBeginPlay
  (bind _returnvalue (PlayerController|LocalPlayerSubsystems|GetEnhancedInputLocalPlayerSubsystem))
  (Utilities|FlowControl|Sequence
    (:then_0
      (Utilities|IsValid _returnvalue
        (:Is%20Valid
          (Input|AddMappingContext _returnvalue "/Game/Project/Input/InputMappingContexts/IMC_Player.IMC_Player" 0 "(bIgnoreAllPressedKeysUntilRelease=True,bForceImmediately=False,bNotifyUserSettings=False)"))))
    (:then_1
      (bind _asbp_player_base (Utilities|Casting|CastToBP_PlayerBase (Pawn|GetControlledPawn)))
      (Variables|Default|SetControlled%20Player _asbp_player_base)
      (CallFunction|InitUI))))

(event EventTick
  (params (DeltaSeconds :type Float%20%28single-precision%29)))

(fn ConstructionScript)