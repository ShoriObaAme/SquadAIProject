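; Base player character with Enhanced Input move, look and jump, tagged at BeginPlay as a combat target for enemies.
; Three formation point components start in a Wedge; SetFormation selects Wedge, Line or Pillar offsets, scaled by FormationRadius.
; Offsets are added to each point's current relative location, so repeated formation changes compound.
; TakeDamage forwards to APCHealthComponent, while the current and max health getters are stubs returning zero.
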(event Input|EnhancedActionEvents|EnhancedInputActionIA_Jump
  (params (ActionValue :type Boolean) (ElapsedSeconds :type Float%20%28double-precision%29) (TriggeredSeconds :type Float%20%28double-precision%29) (InputAction :type Input%20Action%20Object%20Reference :default "/Game/Project/Input/InputActions/Player/IA_Jump.IA_Jump"))
  (:Started
    (Character|Jump))
  (:Completed
    (Character|StopJumping)))

(event Input|EnhancedActionEvents|EnhancedInputActionIA_Movement
  (params (ActionValue :type Vector%202D%20Structure) (ElapsedSeconds :type Float%20%28double-precision%29) (TriggeredSeconds :type Float%20%28double-precision%29) (InputAction :type Input%20Action%20Object%20Reference :default "/Game/Project/Input/InputActions/Player/IA_Movement.IA_Movement"))
  (CallFunction|MovePlayer ActionValue))

(event Input|EnhancedActionEvents|EnhancedInputActionIA_Look
  (params (ActionValue :type Vector%202D%20Structure) (ElapsedSeconds :type Float%20%28double-precision%29) (TriggeredSeconds :type Float%20%28double-precision%29) (InputAction :type Input%20Action%20Object%20Reference :default "/Game/Project/Input/InputActions/Player/IA_Look.IA_Look"))
  (CallFunction|LookPlayer ActionValue))

(event EventBeginPlay
  (Variables|Formations|SetFormation%20Positions (Utilities|Array|MakeArray (Variables|Default|GetFormation%20Pos%20A) (Variables|Default|GetFormation%20Pos%20B) (Variables|Default|GetFormation%20Pos%20C)))
  (CallFunction|SetFormation "NewEnumerator0")
  (GameplayTags|AddGameplayTag (Variables|Default|GetGameplay%20Tag) "(TagName=\"Enemies.Combat.Target\")" :!class /Script/GameplayTags.BlueprintGameplayTagLibrary))

(event Collision|EventActorBeginOverlap
  (params (OtherActor :type Actor%20Object%20Reference)))

(event EventTick
  (params (DeltaSeconds :type Float%20%28single-precision%29)))

(event EventTakeDamage
  (params (Dealt%20Damage :type Float%20%28double-precision%29))
  (Default|TakeDamage (Variables|Default|GetAPC_Health_Component) Dealt%20Damage))

(fn ConstructionScript)

(fn MovePlayer
  (params (Input%20Axes :type Vector%202D%20Structure))
  (bind _returnvalue (Pawn|GetControlRotation :!class /Script/Engine.Pawn))
  (Pawn|Input|AddMovementInput (Math|Vector|GetRightVector (Math|Rotator|MakeRotator (.roll _returnvalue) 0.0 (.yaw _returnvalue))) (.x Input%20Axes) false)
  (Pawn|Input|AddMovementInput (Math|Vector|GetForwardVector (Math|Rotator|MakeRotator 0.0 0.0 (.yaw (Pawn|GetControlRotation :!class /Script/Engine.Pawn)))) (.y Input%20Axes) false))

(fn LookPlayer
  (params (Input%20Axes :type Vector%202D%20Structure))
  (Pawn|Input|AddControllerYawInput (.x Input%20Axes))
  (Pawn|Input|AddControllerPitchInput (.y Input%20Axes)))

(fn SetFormation
  (params (New%20Formation :type E_Formations%20Enum :default "NewEnumerator0"))
  (bind _output_get (Variables|Formations|SetCurrent%20Formation New%20Formation))
  (switch Utilities|FlowControl|Switch|SwitchonE_Formations _output_get
    (:NewEnumerator0
      (CallFunction|UpdateFormationPositions (Variables|Formations|Offsets|GetWedge%20Offsets)))
    (:NewEnumerator1
      (CallFunction|UpdateFormationPositions (Variables|Formations|Offsets|GetLine%20Offsets)))
    (:NewEnumerator2
      (CallFunction|UpdateFormationPositions (Variables|Formations|Offsets|GetPillar%20Offsets)))))

(fn UpdateFormationPositions
  (params (Formation%20Offsets :type Array%20of%20Vectors))
  (bind _formation_radius (Variables|Default|GetFormation%20Radius))
  (for (_array_element _array_index) (Variables|Formations|GetFormation%20Positions)
    (Transformation|SetRelativeLocation _array_element (Math|Vector|MakeVector (.x (* (+ (Variables|/Script/Engine.SceneComponent|GetRelativeLocation _array_element) (Utilities|Array|Get(acopy) Formation%20Offsets _array_index)) (Math|Vector|MakeVector _formation_radius _formation_radius 1.0))) (.y (* (+ (Variables|/Script/Engine.SceneComponent|GetRelativeLocation _array_element) (Utilities|Array|Get(acopy) Formation%20Offsets _array_index)) (Math|Vector|MakeVector _formation_radius _formation_radius 1.0))) (.z (* (+ (Variables|/Script/Engine.SceneComponent|GetRelativeLocation _array_element) (Utilities|Array|Get(acopy) Formation%20Offsets _array_index)) (Math|Vector|MakeVector _formation_radius _formation_radius 1.0)))) false false)))

(fn GetCurrentHealth
  (return 0.0))

(fn GetMaxHealth
  (return 0.0))