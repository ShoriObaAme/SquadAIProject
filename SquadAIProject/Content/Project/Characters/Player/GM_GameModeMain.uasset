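; Main game mode Blueprint that provides hooks for the wave system.
; CreateWaveUIElem, despite its name, spawns a BP_WaveManager and stores it as WaveManager.
; NewWave broadcasts OnWaveBegin with CurrentWave plus one, without storing the new value.
; The wave counter widget creation and initialization nodes are disconnected and never run, and GetHUD is an empty stub.
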(event Custom|New%20Wave
  (Default|CallOnWaveBegin (+ (Variables|Default|GetCurrent%20Wave) 1)))

(event EventCreateWaveUIElem
  (Utilities|FlowControl|Sequence
    (:then_0
      (bind _returnvalue (Game|SpawnActorfromClass "/Game/Project/Blueprints/Gameplay/WaveSystem/BP_WaveManager.BP_WaveManager_C" (Math|Transform|MakeTransform "0, 0, 0" "0, 0, 0" "1.000000,1.000000,1.000000") "Undefined" "MultiplyWithRoot" 0 0))
      (Variables|Default|SetWave%20Manager _returnvalue))))

(fn ConstructionScript)

(fn GMGameModeMainAutoGenFunc
  (params (New%20Wave :type Integer)))

(fn GetHUD
  (return 0))