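; Base character for squad members, controlled by an AIC_SquadMember_Base AI controller.
; On BeginPlay it copies its SquadID to that controller, then adds the Enemies.Combat.Target gameplay tag to its tag container.
; TakeDamage forwards damage to APCHealthComponent, while the current and max health getters are stubs returning zero.
; Tick draws a debug sphere at the pistol weapon socket every frame.
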(event EventBeginPlay
  (bind _asaic_squad_member_base (Utilities|Casting|CastToAIC_SquadMember_Base (AI|GetAIController self)))
  (Variables|/Game/Project/Characters/Squad/AI/Controllers/AIC_SquadMember_Base.AIC_SquadMember_Base_C|SetSquad%20ID _asaic_squad_member_base (Variables|Default|GetSquad%20ID))
  (GameplayTags|AddGameplayTag (Variables|Default|GetGameplay%20Tag) "(TagName=\"Enemies.Combat.Target\")" :!class /Script/GameplayTags.BlueprintGameplayTagLibrary))

(event Collision|EventActorBeginOverlap
  (params (OtherActor :type Actor%20Object%20Reference)))

(event EventTick
  (params (DeltaSeconds :type Float%20%28single-precision%29))
  (Rendering|Debug|DrawDebugSphere (.Location (Math|Transform|BreakTransform (Transformation|GetSocketTransform (Variables|Character|GetMesh) "Weapon_Socket_Pistol" "RTS_World"))) 5.0 6 "(R=1.000000,G=0.000000,B=0.000000,A=1.000000)" 0.25 5.0))

(event EventTakeDamage
  (params (Dealt%20Damage :type Float%20%28double-precision%29))
  (Default|TakeDamage (Variables|Default|GetAPC_Health_Component) Dealt%20Damage))

(fn ConstructionScript)

(fn GetCurrentHealth
  (return 0.0))

(fn GetMaxHealth
  (return 0.0))