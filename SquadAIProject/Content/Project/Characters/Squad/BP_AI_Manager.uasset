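; BP_AI_Manager spawns the player's AI squad when play begins.
; For each requested member, it spawns a BP_SquadMember_Base at the matching formation position on the player character (BP_PlayerBase).
; It then stores the loop index as SquadID on that member's AIC_SquadMember_Base controller.
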(event EventBeginPlay
  (for _index (range 0 (- (Variables|Default|GetSquad%20Members%20To%20Spawn) 1))
    (bind _asbp_player_base (Utilities|Casting|CastToBP_PlayerBase (Game|GetPlayerCharacter 0)))
    (bind _returnvalue (Game|SpawnActorfromClass "/Game/Project/Characters/Squad/BP_SquadMember_Base.BP_SquadMember_Base_C" (Math|Transform|MakeTransform (Transformation|GetWorldLocation (Utilities|Array|Get(acopy) (Variables|/Game/Project/Characters/Player/BP_PlayerBase.BP_PlayerBase_C|GetFormation%20Positions _asbp_player_base) _index)) "0, 0, 0" "1.000000,1.000000,1.000000") "Undefined" "MultiplyWithRoot" 0 0))
    (bind _asaic_squad_member_base (Utilities|Casting|CastToAIC_SquadMember_Base (AI|GetAIController _returnvalue)))
    (Variables|/Game/Project/Characters/Squad/AI/Controllers/AIC_SquadMember_Base.AIC_SquadMember_Base_C|SetSquad%20ID _asaic_squad_member_base _index)))

(event Collision|EventActorBeginOverlap
  (params (OtherActor :type Actor%20Object%20Reference)))

(event EventTick
  (params (DeltaSeconds :type Float%20%28single-precision%29)))

(fn ConstructionScript)