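; BP_Pistol is a hitscan pistol Blueprint that damages whatever its shot hits.
; Its Fire event line-traces on the Visibility channel from the FirePos component to the supplied end point, with persistent debug drawing.
; It sends a fixed damage amount to the hit actor through a TakeDamage interface message, without checking the hit result.
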(event EventBeginPlay
  (|CallParentFunction) ; This node is disabled and will not be called.\nDrag off pins to build functionality.
)

(event Collision|EventActorBeginOverlap
  (params (OtherActor :type Actor%20Object%20Reference))
  (|CallParentFunction OtherActor) ; This node is disabled and will not be called.\nDrag off pins to build functionality.
)

(event EventTick
  (params (DeltaSeconds :type Float%20%28single-precision%29))
  (|CallParentFunction DeltaSeconds) ; This node is disabled and will not be called.\nDrag off pins to build functionality.
)

(event EventFire
  (params (End%20Point :type Vector :default "0, 0, 0"))
  (bind _outhit (Collision|LineTraceByChannel (Transformation|GetWorldLocation (Variables|Default|GetFire%20Pos)) End%20Point "TraceTypeQuery1" false 0 "Persistent" true "(R=1.000000,G=0.000000,B=0.000000,A=1.000000)" "(R=0.000000,G=1.000000,B=0.000000,A=1.000000)" 0.5))
  (Class|IDamageable|TakeDamage(Message) (.HitActor (Collision|BreakHitResult _outhit)) 5.0))

(fn ConstructionScript
  (|CallParentFunction))