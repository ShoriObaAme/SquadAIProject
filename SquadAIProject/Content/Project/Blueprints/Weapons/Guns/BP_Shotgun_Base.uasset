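; Base shotgun weapon Blueprint that fires a spread of hitscan pellets.
; On Fire, it casts one Visibility line trace per pellet from FirePos, in a random direction within a SpreadAngle cone, out to Range.
; Each trace sends a fixed-damage TakeDamage message to the hit actor and draws a one-frame debug line.
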(event EventBeginPlay
  (|CallParentFunction) ; This node is disabled and will not be called.\nDrag off pins to build functionality.
)

(event Collision|EventActorBeginOverlap
  (params (OtherActor :type Actor%20Object%20Reference))
  (|CallParentFunction OtherActor) ; This node is disabled and will not be called.\nDrag off pins to build functionality.
)

(event EventTick
  (params (DeltaSeconds :type Float%20%28single-precision%29))
  (|CallParentFunction DeltaSeconds))

(event EventFire
  (bind _fire_pos (Variables|Default|GetFire%20Pos))
  (bind _returnvalue (Transformation|GetWorldLocation _fire_pos))
  (for _index (range 0 (- (Variables|Default|GetPallet%20Count) 1))
    (bind _outhit (Collision|LineTraceByChannel _returnvalue (+ _returnvalue (* (Class|KismetMathLibrary|RandomUnitVectorinConeinRadians (Math|Vector|GetForwardVector (Variables|Default|GetFire%20Pos)) (Math|Trig|DegreesToRadians (Variables|Default|GetSpread%20Angle))) (Variables|Default|GetRange))) "TraceTypeQuery1" false 0 "ForOneFrame" true "(R=1.000000,G=0.000000,B=0.000000,A=1.000000)" "(R=0.000000,G=0.000000,B=1.000000,A=1.000000)" 1.0))
    (Class|IDamageable|TakeDamage(Message) (.HitActor (Collision|BreakHitResult _outhit)) 26.0)))

(fn ConstructionScript
  (|CallParentFunction))