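; Base weapon pickup actor that shows a floating name widget when the player comes near.
; On BeginPlay it looks up its data table row and passes the weapon name to the widget.
; A sphere overlap by a Player-tagged actor shows the widget and enables Tick, which rotates it toward the player character.
; Any end overlap hides it and stops Tick; no collection logic exists here, only debug prints.
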(event OnComponentBeginOverlap(Sphere1)
  (params (OverlappedComponent :type Primitive%20Component%20Object%20Reference) (OtherActor :type Actor%20Object%20Reference) (OtherComp :type Primitive%20Component%20Object%20Reference) (OtherBodyIndex :type Integer) (bFromSweep :type Boolean) (SweepResult :type Hit%20Result%20Structure%20%28by%20ref%29))
  (if (Actor|ActorHasTag OtherActor "Player")
    (Development|PrintString "PICKUP")
    (Actor|Tick|SetActorTickEnabled true)
    (Rendering|SetVisibility (Variables|Default|GetPickup%20Widget) true false)))

(event OnComponentEndOverlap(Sphere1)
  (params (OverlappedComponent :type Primitive%20Component%20Object%20Reference) (OtherActor :type Actor%20Object%20Reference) (OtherComp :type Primitive%20Component%20Object%20Reference) (OtherBodyIndex :type Integer))
  (Actor|Tick|SetActorTickEnabled false)
  (Rendering|SetVisibility (Variables|Default|GetPickup%20Widget) false false))

(event EventBeginPlay
  (bind _weapon_data_table (Variables|Default|GetWeapon%20Data%20Table))
  (bind _aswb_weapon_pickup (Utilities|Casting|CastToWB_WeaponPickup (UserInterface|GetUserWidgetObject (Variables|Default|GetPickup%20Widget))))
  (bind _returnvalue (Utilities|GetDataTableRow (.datatable _weapon_data_table) (.rowname _weapon_data_table))
    (:then
      (Variables|/Game/Project/UserInterfacce/WorldSpace/WB_WeaponPickup.WB_WeaponPickup_C|SetWeapon%20Name _aswb_weapon_pickup (Utilities|Struct|BreakST_WeaponPickup_Data _returnvalue)))))

(event Collision|EventActorBeginOverlap
  (params (OtherActor :type Actor%20Object%20Reference)))

(event EventTick
  (params (DeltaSeconds :type Float%20%28single-precision%29))
  (Development|PrintString "Hello")
  (Transformation|SetWorldRotation (Variables|Default|GetPickup%20Widget) (Math|Rotator|FindLookatRotation (Transformation|GetActorLocation) (Transformation|GetActorLocation (Game|GetPlayerCharacter 0))) false false))

(fn ConstructionScript)