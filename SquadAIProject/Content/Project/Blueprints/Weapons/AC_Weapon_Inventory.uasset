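; Weapon inventory component that equips its owning Character with a starting weapon on BeginPlay.
; AddWeapon spawns the weapon class, adds it to EquippedWeapons and records it as CurrentWeapon.
; It builds a "Weapon_Socket_" name from TargetSocket, attaches the weapon to that socket's bone on the character mesh, then snaps it to the socket's world transform.
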(event EventBeginPlay
  (CallFunction|AddWeapon (Variables|Default|GetStarting%20Weapon) (Components|GetOwner) (Variables|Default|GetTarget%20Socket)))

(event EventTick
  (params (DeltaSeconds :type Float%20%28single-precision%29)))

(fn AddWeapon
  (params (Weapon%20Class :type BP%20Weapon%20Base%20Class%20Reference) (Owning%20Actor :type Actor%20Object%20Reference) (Target%20Socket :type Name))
  (bind _result (Utilities|Text|FormatText "Weapon_Socket_{Weapon Name}" Target%20Socket))
  (bind _returnvalue (Utilities|String|ToString(Text) _result))
  (bind _returnvalue_2 (Utilities|String|StringToName _returnvalue))
  (bind _ascharacter (Utilities|Casting|CastToCharacter Owning%20Actor))
  (bind _returnvalue_3 (Game|SpawnActorfromClass Weapon%20Class (Math|Transform|MakeTransform "0, 0, 0" "0, 0, 0" "1.000000,1.000000,1.000000") "Undefined" "MultiplyWithRoot" 0 0))
  (Utilities|Array|Add (Variables|Default|GetEquipped%20Weapons) _returnvalue_3)
  (Transformation|AttachComponentToComponent _returnvalue_3 (Variables|/Script/Engine.Character|GetMesh _ascharacter) (Class|SkinnedMeshComponent|GetSocketBoneName (Variables|/Script/Engine.Character|GetMesh _ascharacter) _returnvalue_2) "SnapToTarget" "SnapToTarget" "SnapToTarget" true)
  (Transformation|SetActorTransform _returnvalue_3 (Transformation|GetSocketTransform (Variables|/Script/Engine.Character|GetMesh _ascharacter) _returnvalue_2 "RTS_World"))
  (Variables|Default|SetCurrent%20Weapon _returnvalue_3))