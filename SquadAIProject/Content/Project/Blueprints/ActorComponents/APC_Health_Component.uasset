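; APC_Health_Component is an actor component that tracks health and death for its owning actor.
; BeginPlay fills current health to max and fires the OnDamaged dispatcher with current and max values.
; TakeDamage subtracts damage clamped between zero and max, rebroadcasts OnDamaged, and at zero sets IsDead and sends DieMessage to the owner.
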(event EventBeginPlay
  (bind _max_health (Variables|Default|GetMax%20Health))
  (bind _output_get (Variables|Default|SetCurrent%20Health _max_health))
  (Default|CallOnDamaged _output_get _max_health))

(event EventTick
  (params (DeltaSeconds :type Float%20%28single-precision%29)))

(fn TakeDamage
  (params (Damage%20In :type Float%20%28double-precision%29))
  (bind _output_get (Variables|Default|SetCurrent%20Health (Math|Float|Clamp(Float) (- (Variables|Default|GetCurrent%20Health) Damage%20In) 0.0 (Variables|Default|GetMax%20Health))))
  (Default|CallOnDamaged _output_get (Variables|Default|GetMax%20Health))
  (if (<= (Variables|Default|GetCurrent%20Health) 0.0)
    (Variables|Default|SetbIsDead? true)
    (Class|IDamageable|Die(Message) (Components|GetOwner))))