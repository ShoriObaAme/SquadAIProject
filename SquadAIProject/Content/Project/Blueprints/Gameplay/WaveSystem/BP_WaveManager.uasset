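; Wave manager actor that shows a wave counter on the HUD and announces the first wave at BeginPlay.
; It adds a top-center WB_Wave_Counter to the HUD message canvas, retrying on a short delay until that HUD exists.
; The second sequence branch sets the counter's values and calls NewWave without waiting for that retry.
; NewWave broadcasts OnWaveBegin with the next wave number, clamped to MaxWaves, without updating CurrentWave.
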(event Custom|New%20Wave
  (Default|CallOnWaveBegin (Math|Integer|Clamp(Integer) (+ (Variables|Default|GetCurrent%20Wave) 1) 0 (Variables|Default|GetMax%20Waves))))

(event EventBeginPlay
  (Utilities|FlowControl|Sequence
    (:then_0
      ;[0.15 0.15 0.15 0.5] Create Wave Counter UI Element
      (bind _hud_ref (Class|IGameControl|GetHUD(Message) (Game|GetPlayerController 0) :!label _label))
      (Utilities|IsValid _hud_ref
        (:Is%20Valid
          (bind _returnvalue (UserInterface|CreateWidget "/Game/Project/UserInterfacce/ScreenSpace/Segments/WB_Wave_Counter.WB_Wave_Counter_C" 0 self))
          (bind _output_get (Variables|Default|SetWave%20Counter _returnvalue))
          (bind _returnvalue_2 (Class|CanvasPanel|AddChildtoCanvas (Variables|/Game/Project/UserInterfacce/ScreenSpace/In_Game/WB_InGameUI.WB_InGameUI_C|GetCanvasPanel_42 _hud_ref) _output_get))
          (Class|CanvasPanelSlot|SetSize _returnvalue_2 "(X=250.000000,Y=75.000000)")
          (Class|CanvasPanelSlot|SetAlignment _returnvalue_2 "(X=0.500000,Y=0.000000)")
          (Class|CanvasPanelSlot|SetAnchors _returnvalue_2 (Utilities|Struct|MakeAnchors "(X=0.500000,Y=0.000000)" "(X=0.500000,Y=0.000000)")))
        (:Is%20Not%20Valid
          (Utilities|FlowControl|Delay 0.2)
          (goto _label))))
    (:then_1
      (Variables|/Game/Project/UserInterfacce/ScreenSpace/Segments/WB_Wave_Counter.WB_Wave_Counter_C|SetCurrent%20Wave (Variables|Default|GetWave%20Counter) (Variables|Default|GetCurrent%20Wave))
      (Variables|/Game/Project/UserInterfacce/ScreenSpace/Segments/WB_Wave_Counter.WB_Wave_Counter_C|SetLas%20Wave (Variables|Default|GetWave%20Counter) (Variables|Default|GetMax%20Waves))
      (CallFunction|NewWave))))

(event Collision|EventActorBeginOverlap
  (params (OtherActor :type Actor%20Object%20Reference)))

(event EventTick
  (params (DeltaSeconds :type Float%20%28single-precision%29)))

(fn ConstructionScript)